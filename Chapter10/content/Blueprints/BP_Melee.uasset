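; BP_Melee is an AI-controlled melee actor whose Blueprint provides debug visualization of its behavior.
; A text label shows its display name and turns each tick to face the player pawn.
; An arrow points at the actor stored in a blackboard key and hides when none is set.
; Debug spheres redrawn every tick show the attack and search radii read from the blackboard.
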(event `self.ReceiveBeginPlay`
  (`TextRenderComponent.K2_SetText` (`self.TextRender`) (`KismetTextLibrary.Conv_StringToText` (`KismetSystemLibrary.GetDisplayName` self))))

(event `self.ReceiveTick`
  (params (DeltaSeconds :type "Float (single-precision)"))
  (bind _opponentarrow (`self.OpponentArrow`))
  (`|ExecutionSequence`
    (:`then_0`
      (`SceneComponent.K2_SetWorldRotation` (`self.TextRender`) (`KismetMathLibrary.FindLookAtRotation` (`self.K2_GetActorLocation`) (`self.K2_GetActorLocation` (`GameplayStatics.GetPlayerPawn` 0))) false false)
      (`self.DrawDebug`))
    (:`then_1`
      (bind _asactor (cast `Actor` (`BlackboardComponent.GetValueAsObject` (`AIBlueprintHelperLibrary.GetBlackboard` (`self.GetController`)) (`self.FollowName`)))
        (:`then`
          (`SceneComponent.K2_SetWorldRotation` _opponentarrow (`KismetMathLibrary.FindLookAtRotation` (`self.K2_GetActorLocation`) (`self.K2_GetActorLocation` _asactor)) false false)
          (`SceneComponent.SetVisibility` _opponentarrow true false))
        (:`CastFailed`
          ;[1 1 1] Opponent not set
          (`SceneComponent.SetVisibility` (`self.OpponentArrow`) false false))))))

(fn `DrawDebug`
  (bind _returnvalue (`self.K2_GetActorLocation`))
  (set `self.Blackboard` (`AIBlueprintHelperLibrary.GetBlackboard` null))
  (`|ExecutionSequence`
    (:`then_0`
      (`KismetSystemLibrary.DrawDebugSphere` _returnvalue (`BlackboardComponent.GetValueAsFloat` (`self.Blackboard`) (`self.AttackRadiusName`)) 12 (struct :`R` 1.0 :`G` 0.732847 :`A` 1.0) 0.0))
    (:`then_1`
      (`KismetSystemLibrary.DrawDebugSphere` _returnvalue (`BlackboardComponent.GetValueAsFloat` (`self.Blackboard`) (`self.SearchRadiusName`)) 12 (struct :`R` 1.0 :`G` 1.0 :`B` 1.0 :`A` 1.0) 0.0))))

(fn `UserConstructionScript`)