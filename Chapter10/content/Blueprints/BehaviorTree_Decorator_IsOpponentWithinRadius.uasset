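; Behavior tree decorator that checks whether the AI's follow target is within its attack radius.
; It reads target and radius from the Blackboard, then sphere-overlaps Pawn-type Characters around the controlled pawn, ignoring itself, and tests whether the target is among them.
; A red debug sphere shows the radius.
; A missing target logs an error and jumps straight to the return, before the overlap runs.
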(fn `PerformConditionCheckAI`
  (params (OwnerController :type "AIController Object Reference") (ControlledPawn :type "Pawn Object Reference"))
  (returns (ReturnValue :type Boolean))
  (bind _returnvalue (`Actor.K2_GetActorLocation` ControlledPawn))
  (bind _returnvalue_2 (`BlackboardComponent.GetValueAsFloat` (`self.Blackboard`) (`self.AttackRadiusName`)))
  (`|ExecutionSequence`
    (:`then_0`
      (set `self.Blackboard` (`AIBlueprintHelperLibrary.GetBlackboard` OwnerController)))
    (:`then_1`
      (bind _asactor (cast `Actor` (`BlackboardComponent.GetValueAsObject` (`self.Blackboard`) (`self.FollowName`)))
        (:`then`
          (set `self.FollowTarget` _asactor))
        (:`CastFailed`
          (`/Game/Blueprints/Functions.Error` "Follow had no target")
          (return (`KismetArrayLibrary.Array_Contains` (stale _outactors) (`self.FollowTarget`))))))
    (:`then_2`
      (`KismetSystemLibrary.DrawDebugSphere` _returnvalue _returnvalue_2 12 (struct :`R` 1.0 :`A` 1.0)))
    (:`then_3`
      (bind _outactors (`KismetSystemLibrary.SphereOverlapActors_NEW` _returnvalue _returnvalue_2 (`|MakeArray` "ObjectTypeQuery3" :!type "EObjectTypeQuery Enum") "/Script/Engine.Character" (`|MakeArray` ControlledPawn :!type "Actor Object Reference")))
      (return (`KismetArrayLibrary.Array_Contains` _outactors (`self.FollowTarget`))))))