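; Behavior tree service that picks the nearest Character as a melee AI's opponent.
; Each tick it reads a search radius from the Blackboard and sphere-overlaps Pawns around the controlled pawn, excluding itself.
; GetClosest linearly scans the hits by distance, and the result is written to the Blackboard follow key.
; Any Character qualifies, with no team or line-of-sight check.
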(event EventReceiveTickAI
  (params (OwnerController :type AI%20Controller%20Object%20Reference) (ControlledPawn :type Pawn%20Object%20Reference) (DeltaSeconds :type Float%20%28single-precision%29))
  (Utilities|FlowControl|Sequence
    (:then_0
      ;[1 1 1] 1. Set Attacker & Get the Blackboard
      (Variables|Default|SetAttacker ControlledPawn)
      (Variables|Default|SetBlackboard (AI|GetBlackboard OwnerController)))
    (:then_1
      ;[1 1 1] 2. Get the search radius
      (Variables|Default|SetSearchRadius (Class|BlackboardComponent|GetValueasFloat (Variables|Default|GetBlackboard) (Variables|Default|GetSearchRadiusName))))
    (:then_2
      ;[1 1 1] 3. Get nearest Character in bounding sphere
      (bind _outactors (Class|KismetSystemLibrary|SphereOverlapActorsNEW (Transformation|GetActorLocation (Variables|Default|GetAttacker)) (Variables|Default|GetSearchRadius) (Utilities|Array|MakeArray "ObjectTypeQuery3") "/Script/Engine.Character" (Utilities|Array|MakeArray (Variables|Default|GetAttacker))))
      (bind _outactor (CallFunction|GetClosest _outactors (Variables|Default|GetAttacker)))
      (bind _output_get (Variables|Default|SetFollowTarget _outactor))
      (AI|Components|Blackboard|SetValueasObject (Variables|Default|GetBlackboard) (Variables|Default|GetFollowName) _output_get))))

(fn GetClosest
  (params (Actors :type Array%20of%20Actor%20Object%20References) (InActor :type Actor%20Object%20Reference))
  (Utilities|FlowControl|Sequence
    (:then_0
      ;[1 1 1] 1. Set this (searching) actor
      (LocalVariables|SetThisActor InActor))
    (:then_1
      ;[1 1 1] 2. If there are 0 array elts, then end (no closest)
      (if (<= (Utilities|Array|Length Actors) 0)
        (return 0)))
    (:then_2
      ;[1 1 1] 3. Start with Closest as elt 0, to initialize ClosestDistance. Array has size due to check above.
      (bind _output_get (LocalVariables|SetClosest (Utilities|Array|Get(acopy) Actors)))
      (LocalVariables|SetClosestDistance (Transformation|GetDistanceTo (Variables|Default|GetAttacker) _output_get)))
    (:then_3
      ;[1 1 1] 4. Loop: Distance to new Actor less than closest so far
      (for _array_element Actors
        (Variables|Default|SetNewActor _array_element)
        (if (< (Transformation|GetDistanceTo (LocalVariables|GetThisActor) (Variables|Default|GetNewActor)) (LocalVariables|GetClosestDistance))
          (LocalVariables|SetClosest (Variables|Default|GetNewActor))
          (LocalVariables|SetClosestDistance (Transformation|GetDistanceTo (LocalVariables|GetThisActor) (Variables|Default|GetNewActor)))))
      (return (LocalVariables|GetClosest)))))