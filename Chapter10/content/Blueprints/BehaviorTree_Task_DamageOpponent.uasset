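; Behavior Tree task in which an AI pawn damages the actor it is following.
; It reads the follow target and attack damage from the controller's Blackboard, then calls ApplyDamage with the pawn as damage causer.
; It finishes successfully and logs the hit.
; A failed target cast logs an error and finishes as failed, but the later sequence steps still run.
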(event `self.ReceiveExecuteAI`
  (params (OwnerController :type "AIController Object Reference") (ControlledPawn :type "Pawn Object Reference"))
  (`|ExecutionSequence`
    (:`then_0`
      ;[1 1 1] 1. Get the Blackboard for this Attacker
      (set `self.Blackboard` (`AIBlueprintHelperLibrary.GetBlackboard` OwnerController))
      (set `self.Attacker` ControlledPawn))
    (:`then_1`
      ;[1 1 1] 2. Get the follow target
      (bind _asactor (cast `Actor` (`BlackboardComponent.GetValueAsObject` (`self.Blackboard`) (`self.FollowName`)))
        (:`then`
          (set `self.FollowTarget` _asactor))
        (:`CastFailed`
          ;[1 1 1] If there's no Follow, exit with fail
          (`/Game/Blueprints/Functions.Error` "BT_Task_DamageOpponent: Failed to cast Follow to actor")
          (`self.FinishExecute` false))))
    (:`then_2`
      ;[1 1 1] 3. Get attack damage
      (set `self.AttackDamage` (`BlackboardComponent.GetValueAsFloat` (`self.Blackboard`) (`self.AttackDamageName`))))
    (:`then_3`
      ;[1 1 1] 4. Apply the damage
      (`GameplayStatics.ApplyDamage` (`self.FollowTarget`) (`self.AttackDamage`) null (`self.Attacker`))
      (`|ExecutionSequence`
        (:`then_0`
          (`self.FinishExecute` true))
        (:`then_1`
          ;[1 1 1] Print damage
          (`/Game/Blueprints/Functions.Info` "TaskDamage" (`|FormatText` "{Actor1} Damaging opponent {Actor2} for {damage} units of damage" (`/Game/Blueprints/ObjectMacroLibrary.GetActorName` (`self.Attacker`)) (`/Game/Blueprints/ObjectMacroLibrary.GetActorName` (`self.FollowTarget`)) (`KismetTextLibrary.Conv_DoubleToText` (`self.AttackDamage`) "HalfToEven"))))))))