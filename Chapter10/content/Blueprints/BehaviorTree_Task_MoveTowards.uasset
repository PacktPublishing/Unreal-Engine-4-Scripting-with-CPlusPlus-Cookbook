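; Behavior Tree task that moves the AI pawn incrementally towards its Blackboard follow target.
; On AI tick it reads the target Actor, failing the task if the cast fails, then calls AI MoveTo with half the Blackboard attack radius as acceptance radius.
; It finishes successfully as soon as the move is issued rather than waiting for arrival; the debug print for blocked moves is disconnected.
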(event `self.ReceiveTickAI`
  (params (OwnerController :type "AIController Object Reference") (ControlledPawn :type "Pawn Object Reference") (DeltaSeconds :type "Float (single-precision)"))
  (`|ExecutionSequence`
    (:`then_0`
      ;[1 1 1] 1. Get the Controller's Blackboard, and the Moving Pawn ref
      (set `self.Blackboard` (`AIBlueprintHelperLibrary.GetBlackboard` OwnerController))
      (set `self.MovingPawn` ControlledPawn))
    (:`then_1`
      ;[1 1 1] 2. Get the Pawn's Follow target from the Blackboard
      (bind _asactor (cast `Actor` (`BlackboardComponent.GetValueAsObject` (`self.Blackboard`) (`self.FollowName`)))
        (:`then`
          (set `self.FollowTarget` _asactor))
        (:`CastFailed`
          (`/Game/Blueprints/Functions.Error` "BT_Task_MoveTowards: Blackboard Follow target failed to cast to Actor")
          ;;[1 1 1] Function failed when cast fails
          (`self.FinishExecute` false))))
    (:`then_2`
      ;[1 1 1] 3. Move an incremental amount towards the Follow target
      (bind _movementresult (`|AIMoveTo` (`self.MovingPawn`) (0.0 0.0 0.0) (`self.FollowTarget`) (/ (`BlackboardComponent.GetValueAsFloat` (`self.Blackboard`) (`self.AttackRadiusName`)) 2.0))
        (:`then`
          _)
        (:`OnSuccess`
          _))
      (`self.FinishExecute` true))))