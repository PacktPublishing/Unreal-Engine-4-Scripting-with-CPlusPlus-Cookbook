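; Blueprint function collection of debug helpers that print formatted on-screen messages.
; Basic printers show floats, text and strings for ten seconds, and the Blackboard variants look up float or string values by key name to print them.
; Error, Warning and Info join a string and text in red, yellow or white with optional duration.
; Warning prints only when the supplied duration is not positive.
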(fn PrintFloat
  (params (string :type String) (FData :type Float%20%28single-precision%29))
  (Development|PrintString 0 (Utilities|String|ToString(Text) (Utilities|Text|FormatText "{name} = {data}" (Utilities|Text|ToText(String) string) (Utilities|Text|ToText(Float) FData "HalfToEven"))) true true "(R=0.000000,G=0.660000,B=1.000000,A=1.000000)" 1e+01)
  (return))

(fn PrintText
  (params (text :type Text))
  (Development|PrintString 0 (Utilities|String|ToString(Text) text) true true "(R=0.000000,G=0.660000,B=1.000000,A=1.000000)" 1e+01)
  (return))

(fn PrintString
  (params (VariableName :type Text))
  (Development|PrintString 0 (Utilities|String|ToString(Text) VariableName) true true "(R=0.000000,G=0.660000,B=1.000000,A=1.000000)" 1e+01)
  (return))

(fn PrintBlackboardFloat
  (params (Blackboard :type Blackboard%20Component%20Object%20Reference) (ParameterName :type String))
  (CallFunction|PrintFloat ParameterName (Class|BlackboardComponent|GetValueasFloat Blackboard (Utilities|String|StringToName ParameterName))))

(fn PrintBlackboardString
  (params (Blackboard :type Blackboard%20Component%20Object%20Reference) (ParameterName :type String))
  (CallFunction|PrintString (Utilities|Text|FormatText "BB Param {ParamName} = {ParamValue}" (Utilities|Text|ToText(String) ParameterName) (Utilities|Text|ToText(String) (Class|BlackboardComponent|GetValueasString Blackboard (Utilities|String|StringToName ParameterName))))))

(fn Error
  (params (MessageAsString :type String) (MessageAsText :type Text) (FDuration :type Float%20%28single-precision%29))
  (if (> FDuration 0.0)
    (LocalVariables|SetVarDuration FDuration))
  (Development|PrintString 0 (Utilities|String|ToString(Text) (Utilities|Text|FormatText "{STRING}{TEXT}" (Utilities|Text|ToText(String) MessageAsString) MessageAsText)) true true "(R=1.000000,G=0.000000,B=0.000000,A=1.000000)" (LocalVariables|GetVarDuration)))

(fn Warning
  (params (MessageAsString :type String) (MessageAsText :type Text) (FDuration :type Float%20%28single-precision%29))
  (if (> FDuration 0.0)
    (LocalVariables|SetTheDuration FDuration)
    (else
      (Development|PrintString 0 (Utilities|String|ToString(Text) (Utilities|Text|FormatText "{STRING}{TEXT}" (Utilities|Text|ToText(String) MessageAsString) MessageAsText)) true true "(R=1.000000,G=1.000000,B=0.000000,A=1.000000)" (LocalVariables|GetTheDuration)))))

(fn Info
  (params (MessageAsString :type String) (MessageAsText :type Text) (FDuration :type Float%20%28single-precision%29))
  (if (> FDuration 0.0)
    (LocalVariables|SetVarDuration FDuration))
  (Development|PrintString 0 (Utilities|String|ToString(Text) (Utilities|Text|FormatText "{STRING}{TEXT}" (Utilities|Text|ToText(String) MessageAsString) MessageAsText)) true true "(R=1.000000,G=1.000000,B=1.000000,A=1.000000)" (LocalVariables|GetVarDuration)))